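; Energy ball projectile, named as the rightward shot of the tower bomb, that damages what it hits.
; On BeginPlay its ProjectileMovement sends it along local Y at the Velocidade speed.
; On sphere overlap it is destroyed by "Barreira" actors.
; Otherwise it removes one Health from a BlocoDestrutivo tagged "Inimigo" or an untagged BP_BomberMago, then destroys itself; other actors are ignored.
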(event OnComponentBeginOverlap(Sphere)
  (params (OverlappedComponent :type Primitive%20Component%20Object%20Reference) (OtherActor :type Actor%20Object%20Reference) (OtherComp :type Primitive%20Component%20Object%20Reference) (OtherBodyIndex :type Integer) (bFromSweep :type Boolean) (SweepResult :type Hit%20Result%20Structure%20%28by%20ref%29))
  ;[1 1 1] Sistema de Dano
  (if (Actor|ActorHasTag OtherActor "Barreira")
    (Actor|DestroyActor)
    (elif (Actor|ActorHasTag OtherActor "Inimigo")
      (bind _asbloco_destrutivo (Utilities|Casting|CastToBlocoDestrutivo OtherActor))
      (Variables|/Game/Marcos/Mesh/BlocoDestrutivo.BlocoDestrutivo_C|Sethealth _asbloco_destrutivo (- (Variables|/Game/Marcos/Mesh/BlocoDestrutivo.BlocoDestrutivo_C|Gethealth _asbloco_destrutivo) 1.0))
      (Actor|DestroyActor)
      (else
        (bind _asbp_bomber_mago (Utilities|Casting|CastToBP_BomberMago OtherActor))
        (Variables|/Game/Marcos/Blueprints/BP_BomberMago.BP_BomberMago_C|SetHealth _asbp_bomber_mago (- (Variables|/Game/Marcos/Blueprints/BP_BomberMago.BP_BomberMago_C|GetHealth _asbp_bomber_mago) 1.0))
        (Actor|DestroyActor)))))

(event EventBeginPlay
  ;[1 1 1] Sistema de Dano
  (Game|Components|ProjectileMovement|SetVelocityinLocalSpace (Variables|Default|GetProjectileMovement) (Math|Vector|MakeVector 0.0 (Variables|Default|GetVelocidade) 0.0)))

(fn ConstructionScript)