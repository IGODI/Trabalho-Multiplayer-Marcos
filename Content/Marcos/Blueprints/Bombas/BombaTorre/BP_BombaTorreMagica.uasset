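; BP_BombaTorreMagica is a magic tower bomb that bursts into four energy balls shortly after it spawns.
; On BeginPlay it waits briefly, then spawns front, back, left and right energy ball actors at its ParticleSystem transform.
; Each ball receives the Velocidade speed, negated for back and left, and the bomb destroys itself a moment later.
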(event EventBeginPlay
  (bind _velocidade (Variables|Default|Getvelocidade))
  (bind _particlesystem (Variables|Default|GetParticleSystem))
  (bind _returnvalue (Transformation|GetWorldTransform _particlesystem))
  ;[1 1 1] Sistema de Spawn de FX
  (Utilities|FlowControl|Delay 1.0)
  (Game|SpawnActorfromClass "/Game/Marcos/Blueprints/Bombas/BombaTorre/BP_BoladeEnergiaFrente.BP_BoladeEnergiaFrente_C" _returnvalue "Undefined" 0 _velocidade 0)
  (Game|SpawnActorfromClass "/Game/Marcos/Blueprints/Bombas/BombaTorre/BP_BoladeEnergiaTras.BP_BoladeEnergiaTras_C" _returnvalue "Undefined" 0 (* _velocidade -1.0) 0)
  (Game|SpawnActorfromClass "/Game/Marcos/Blueprints/Bombas/BombaTorre/BP_BoladeEnergiaEsquerda.BP_BoladeEnergiaEsquerda_C" _returnvalue "Undefined" 0 (* _velocidade -1.0) 0)
  (Game|SpawnActorfromClass "/Game/Marcos/Blueprints/Bombas/BombaTorre/BP_BoladeEnergiaDireita.BP_BoladeEnergiaDireita_C" _returnvalue "Undefined" 0 _velocidade 0)
  (Utilities|FlowControl|Delay 0.1)
  (Actor|DestroyActor))

(fn ConstructionScript)