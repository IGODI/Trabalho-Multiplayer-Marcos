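; Magic bomb actor that detonates on a one-second fuse after it spawns, producing a cross-shaped explosion.
; BeginPlay waits, then spawns front, back, left and right explosion actors at fixed world-axis offsets from the particle system before destroying the bomb.
; Each explosion receives the bomb's Força value, while only the back and left spawns set an explicit Direção, leaving the other two on their defaults.
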(event EventBeginPlay
  (bind _particlesystem (Variables|Default|GetParticleSystem))
  (bind _returnvalue (Transformation|GetWorldLocation _particlesystem))
  ;[1 1 1] Sistema de Spawn de FX
  (Utilities|FlowControl|Delay 1.0)
  (Game|SpawnActorfromClass "/Game/Marcos/Blueprints/Bombas/BombaPadrão/ExplosãoFrente.ExplosãoFrente_C" (Math|Transform|MakeTransform (+ _returnvalue "100.000000, 0, 0") "0, 0, 0" "1,1,1") "Undefined" 0 (Variables|Default|GetForça) "1.000000,0.000000,0.000000" 0)
  (Game|SpawnActorfromClass "/Game/Marcos/Blueprints/Bombas/BombaPadrão/ExplosãoTras.ExplosãoTras_C" (Math|Transform|MakeTransform (+ _returnvalue "-100.000000,0.000000, 0") "0, 0, 0" "1,1,1") "Undefined" 0 (Variables|Default|GetForça) "-1.000000,0.000000,0.000000" 0)
  (Game|SpawnActorfromClass "/Game/Marcos/Blueprints/Bombas/BombaPadrão/ExplosãoEsquerda.ExplosãoEsquerda_C" (Math|Transform|MakeTransform (+ _returnvalue "0,-100.000000, 0") "0, 0, 0" "1,1,1") "Undefined" 0 (Variables|Default|GetForça) "0.000000,-1.000000,0.000000" 0)
  (Game|SpawnActorfromClass "/Game/Marcos/Blueprints/Bombas/BombaPadrão/ExplosãoDireita.ExplosãoDireita_C" (Math|Transform|MakeTransform (+ _returnvalue "0,100.000000, 0") "0, 0, 0" "1,1,1") "Undefined" 0 (Variables|Default|GetForça) "0.000000,1.000000,0.000000" 0)
  (Actor|DestroyActor))

(fn ConstructionScript)